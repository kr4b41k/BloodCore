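; DP_Movement is a player character Blueprint that provides basic walking, camera look and double jump.
; Movement axis inputs feed movement along the actor's forward (X axis) and right (Y axis) vectors.
; Camera axis inputs are scaled down and applied as controller yaw and pitch.
; Space Bar is bound directly to Jump, with the second jump enabled by raising the max jump count on BeginPlay.
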(event `self.ReceiveBeginPlay`
  (set `self.JumpMaxCount` 2))

(event `InputAxis|Camera_MovementAxisX`
  (params (AxisValue :type "Float (single-precision)"))
  (`self.AddControllerYawInput` (* AxisValue 0.4)))

(event `InputAxis|MovementAxisX`
  (params (AxisValue :type "Float (single-precision)"))
  (`self.AddMovementInput` (`self.GetActorForwardVector`) AxisValue))

(event `InputAxis|Camera_MovementAxisY`
  (params (AxisValue :type "Float (single-precision)"))
  (`self.AddControllerPitchInput` (* AxisValue 0.4)))

(event `InputAxis|MovementAxisY`
  (params (AxisValue :type "Float (single-precision)"))
  (`self.AddMovementInput` (`self.GetActorRightVector`) AxisValue))

(event `Key|SpaceBar`
  (params (Key :type "Key Structure"))
  (:`Pressed`
    (`self.Jump`)))

(fn `UserConstructionScript`
  (`parent.UserConstructionScript`))