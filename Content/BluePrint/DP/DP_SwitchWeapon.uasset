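; DP_SwitchWeapon switches the active weapon's data by loading a named row from the WeaponsData table.
; SetWeapon stores the found row and calls CE_SetWeapon, whose SRW graph copies each field into separate variables for combat stats, audio, visuals and attachment.
; RemoveWeapon finds actors of the stored weapon class and destroys the first, returning from inside the loop.
; No actor spawning happens here.
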(event `self.ReceiveBeginPlay`
  (`parent.ReceiveBeginPlay`))

(event `CE_SetWeapon`
  (bind (_out_row_damage _out_row_distance _out_row_rateoffire _out_row_alternativedamage _out_row_distancerange _out_row_recoilrange _out_row_spreading _out_row_wb_texture _out_row_sprite _out_row_sound _out_row_alternative_sound _out_row_shothole _out_row_ballistic_ _out_row_doublehand_ _out_row_issprite_ _out_row_name _out_row_bonename _out_row_actor _out_row_shootcamshake) (break `/Game/BluePrint/Weapon/WeaponSettings` (`self.Out Row`)))
  (`|ExecutionSequence`
    (:`then_0`
      (set `self.Out Row   Damage` _out_row_damage))
    (:`then_1`
      (set `self.Out Row   Distance` _out_row_distance))
    (:`then_2`
      (set `self.Out Row   Rate Of Fire` _out_row_rateoffire))
    (:`then_3`
      (set `self.Out Row   Alternative Damage` _out_row_alternativedamage))
    (:`then_4`
      (set `self.Out Row   Distance Range` _out_row_distancerange))
    (:`then_5`
      (set `self.Out Row   Recoil Range` _out_row_recoilrange))
    (:`then_6`
      (set `self.Out Row   Spreading` _out_row_spreading))
    (:`then_7`
      (set `self.Out Row   WB Texture` _out_row_wb_texture))
    (:`then_8`
      (set `self.Out Row   Sound` _out_row_sound))
    (:`then_9`
      (set `self.Out Row Sprite` _out_row_sprite))
    (:`then_10`
      (set `self.Out Row   Alternative Sound` _out_row_alternative_sound))
    (:`then_11`
      (set `self.Out Row   Shot Hole` _out_row_shothole))
    (:`then_12`
      (set `self.Out Row    Ballistic?` _out_row_ballistic_))
    (:`then_13`
      (set `self.Out Row    Double Hand?` _out_row_doublehand_))
    (:`then_14`
      (set `self.Out Row Is Sprite?` _out_row_issprite_))
    (:`then_15`
      (set `self.Out Row   Name` _out_row_name))
    (:`then_16`
      (set `self.Out Row   Bone Name` _out_row_bonename))
    (:`then_17`
      (set `self.Out Row   Actor` _out_row_actor))
    (:`then_18`
      (set `self.Out Row   Shoot Cam Shake` _out_row_shootcamshake))))

(fn `RemoveWeapon`
  (returns (ReturnValue :type Boolean))
  (bind _outactors (`GameplayStatics.GetAllActorsOfClass` (`self.Out Row   Actor`)))
  (for _array_element _outactors
    (`self.K2_DestroyActor` _array_element)
    (return true)))

(fn `SetWeapon`
  (params (Row :type Name))
  (returns (ReturnValue :type Boolean))
  (bind _returnvalue (`|GetDataTableRow` "/Game/BluePrint/Weapon/WeaponsData.WeaponsData" Row)
    (:`then`
      (set `self.Out Row` _returnvalue)
      (`self.CE_SetWeapon`)
      (return true))))

(fn `UserConstructionScript`
  (`parent.UserConstructionScript`))