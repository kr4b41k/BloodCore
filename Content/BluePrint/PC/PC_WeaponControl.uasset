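; Player controller Blueprint that switches between five weapon slots using Enhanced Input actions, selecting the first slot shortly after BeginPlay.
; SetRow looks up the slot's row name in WPRowArrow and, when it differs from the previous one, triggers weapon removal, then setting.
; Both events broadcast through BPI_DP_SwitchWeapon to every implementing actor, passing the new row on set.
; A collapsed graph prints last and current rows for debugging.
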(event `self.ReceiveBeginPlay`
  (`parent.ReceiveBeginPlay`)
  (`KismetSystemLibrary.Delay` 0.2)
  (`self.SetRow` 0))

(event `PC_SetWeapon`
  (bind _outactors (`GameplayStatics.GetAllActorsWithInterface` "/Game/BluePrint/DP/BPI/BPI_DP_SwitchWeapon.BPI_DP_SwitchWeapon_C"))
  (for _array_element _outactors
    (message `/Game/BluePrint/DP/BPI/BPI_DP_SwitchWeapon.SetWeapon` _array_element (`self.Row`))))

(event `EnhancedInput|/Game/BluePrint/IMC/IA/IA_WP_First`
  (params (ActionValue :type Boolean) (ElapsedSeconds :type "Float (double-precision)") (TriggeredSeconds :type "Float (double-precision)") (InputAction :type "InputAction Object Reference" :default "/Game/BluePrint/IMC/IA/IA_WP_First.IA_WP_First"))
  (:`Triggered`
    (`self.SetRow` 0)))

(event `PC_RemoveWeapon`
  (bind _outactors (`GameplayStatics.GetAllActorsWithInterface` "/Game/BluePrint/DP/BPI/BPI_DP_SwitchWeapon.BPI_DP_SwitchWeapon_C"))
  (for _array_element _outactors
    (message `/Game/BluePrint/DP/BPI/BPI_DP_SwitchWeapon.RemoveWeapon` _array_element)))

(event `EnhancedInput|/Game/BluePrint/IMC/IA/IA_WP_Second`
  (params (ActionValue :type Boolean) (ElapsedSeconds :type "Float (double-precision)") (TriggeredSeconds :type "Float (double-precision)") (InputAction :type "InputAction Object Reference" :default "/Game/BluePrint/IMC/IA/IA_WP_Second.IA_WP_Second"))
  (:`Triggered`
    (`self.SetRow` 1)))

(event `EnhancedInput|/Game/BluePrint/IMC/IA/IA_WP_Third`
  (params (ActionValue :type Boolean) (ElapsedSeconds :type "Float (double-precision)") (TriggeredSeconds :type "Float (double-precision)") (InputAction :type "InputAction Object Reference" :default "/Game/BluePrint/IMC/IA/IA_WP_Third.IA_WP_Third"))
  (:`Triggered`
    (`self.SetRow` 2)))

(event `EnhancedInput|/Game/BluePrint/IMC/IA/IA_WP_Fourth`
  (params (ActionValue :type Boolean) (ElapsedSeconds :type "Float (double-precision)") (TriggeredSeconds :type "Float (double-precision)") (InputAction :type "InputAction Object Reference" :default "/Game/BluePrint/IMC/IA/IA_WP_Fourth.IA_WP_Fourth"))
  (:`Triggered`
    (`self.SetRow` 3)))

(event `EnhancedInput|/Game/BluePrint/IMC/IA/IA_WP_Fifth`
  (params (ActionValue :type Boolean) (ElapsedSeconds :type "Float (double-precision)") (TriggeredSeconds :type "Float (double-precision)") (InputAction :type "InputAction Object Reference" :default "/Game/BluePrint/IMC/IA/IA_WP_Fifth.IA_WP_Fifth"))
  (:`Triggered`
    (`self.SetRow` 4)))

(fn `SetRow`
  (params (`Dimension 1` :type Integer))
  (bind _output_get (set `self.LastRow` (`self.Row`)))
  (bind _output_get_2 (set `self.Row` (`|GetArrayItem` (`self.WP_Row_Arrow`) `Dimension 1`)))
  (`KismetSystemLibrary.PrintString` (`KismetStringLibrary.Concat_StrStr` (`KismetStringLibrary.Conv_NameToString` _output_get) " Last") true true (struct :`R` 1.0 :`G` 0.401145 :`A` 1.0))
  (if (not (== _output_get _output_get_2))
    (`KismetSystemLibrary.PrintString` (`KismetStringLibrary.Concat_StrStr` (`KismetStringLibrary.Conv_NameToString` _output_get_2) " Current") true true (struct :`R` 1.0 :`B` 0.133291 :`A` 1.0))
    (if (!= (`self.LastRow`) (`self.Row`))
      (`self.PC_RemoveWeapon`)
      (`self.PC_SetWeapon`))))

(fn `UserConstructionScript`
  (`parent.UserConstructionScript`))